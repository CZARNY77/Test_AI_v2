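; BP_AI_NPC is a voice-driven AI NPC that turns recorded speech into a spoken chatbot reply.
; Audio capture records through a submix to a WAV file, which OpenAI transcribes and appends to a running chat log.
; GPT-3.5 Turbo answers from that log, and text-to-speech plays the reply using the ConvaiChatbot voice.
; The API key comes from environment variables; ContextDetection is an empty, unconnected stub.
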(event Custom|StopRecording
  ;[1 1 1] Recording
  (Audio|Components|Audio|Stop (Variables|Default|GetAudioCapture))
  (Class|AudioMixerBlueprintLibrary|StopRecordingOutput "WavFile" (Variables|Default|GetFileName) "" (Variables|Default|GetMySubmix) 0)
  (EventDispatchers|AssignOnSubmixRecordedFileDone (Variables|Default|GetMySubmix) (delegate Custom|SoundToText)))

(event Custom|StartRecording
  ;[1 1 1] Recording
  (CameraShake|Start (Variables|Default|GetAudioCapture))
  (Development|PrintString "Start")
  (Class|AudioMixerBlueprintLibrary|StartRecordingOutput 5.0 (Variables|Default|GetMySubmix)))

(event Custom|SendPrompt
  (params (ChatLog :type Chat%20Log%20Structure))
  ;[1 1 1] Send Prompt
  (Utilities|Array|Add (Variables|Default|GetChatLog) ChatLog)
  (bind (_message _errormessage _success) (|OpenAICallChat (Utilities|Struct|MakeChatSettings "GPT_3_5_TURBO" (Variables|Default|GetChatLog) 0.7 150))
    (:Finished
      (if _success
        (Utilities|Array|Add (Variables|Default|GetChatLog) (.message (Utilities|Struct|BreakChatCompletion _message)))
        (Utilities|String|LogString (Utilities|String|Append "ASSISTANT: " (.content (Utilities|Struct|BreakChatLog (.message (Utilities|Struct|BreakChatCompletion _message))))))
        (CallFunction|TexttoSound (.content (Utilities|Struct|BreakChatLog (.message (Utilities|Struct|BreakChatCompletion _message)))))
        (else
          (Development|PrintString _errormessage))))))

(event Custom|SoundToText
  (params (ResultingSoundWave :type Sound%20Wave%20Object%20Reference))
  ;[1 1 1] Sound To Text
  (Development|PrintString "Konwertuje")
  (bind (_transcription _errormessage _success) (|OpenAICallTranscriptions (Variables|Default|GetFileName))
    (:Finished
      (if _success
        (Utilities|String|LogString (Utilities|String|Append "USER: " _transcription))
        (CallFunction|SendPrompt (Utilities|Struct|MakeChatLog "USER" _transcription))
        (else
          (Development|PrintString _errormessage))))))

(event Custom|TextToSound
  (params (Content :type String))
  (bind _convaichatbot (Variables|Default|GetConvaiChatbot))
  (bind _wave (|TexttoSpeechQueryProxy Content (Variables|/Script/Convai.ConvaiChatbotComponent|GetVoiceType (Variables|Default|GetConvaiChatbot)))
    (:OnSuccess
      (Audio|Components|Audio|SetSound _convaichatbot _wave)
      (Audio|Components|Audio|Play _convaichatbot 0.0))
    (:OnFailure
      (Utilities|String|LogString "Error text to speech"))))

(event Custom|TestSound
  (Audio|Components|Audio|SetSound (Variables|Default|GetAudio) (Variables|Default|GetMySound))
  (Audio|Components|Audio|SetSubmixSend (Variables|Default|GetAudio) (Variables|Default|GetMySubmix) 0.5 :!class /Script/Engine.AudioComponent)
  (Audio|Components|Audio|Play (Variables|Default|GetAudio) 0.0))

(event EventBeginPlay
  (Class|OpenAIUtils|SetUseOpenAIApiKeyfromEnvironmentVars true))

(fn ConstructionScript)

(fn ContextDetection
  (params (Content :type String)))